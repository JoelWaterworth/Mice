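; BPlib holds a path reconstruction helper, CameFromToPath, of the kind used after a graph search such as A*.
; It starts at the given node and follows predecessor links in the input map until a node has no entry.
; Each visited node is added to the returned CameFrom array, which runs from the given node back to the origin without being reversed.
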(fn CamefromtoPath
  (params (N_current :type Vector%202D%20Int%20Structure) (InputPin :type Map%20of%20Vector%202D%20Int%20Structures%20to%20Structs))
  (bind _output_get (LocalVariables|Setcurrent N_current))
  (Utilities|Array|Add (LocalVariables|GetcameFrom) _output_get)
  (while (Utilities|Map|Contains InputPin (LocalVariables|Getcurrent))
    (bind _output_get_2 (LocalVariables|Setcurrent (.Value (Utilities|Map|Find InputPin (LocalVariables|Getcurrent)))))
    (Utilities|Array|Add (LocalVariables|GetcameFrom) _output_get_2))
  (return (LocalVariables|GetcameFrom)))