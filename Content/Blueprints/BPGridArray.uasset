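; Grid structure actor that builds a turtle-style path of pieces from a list of turn directions in its construction script.
; Each step advances a grid cell, turns, and records cell data from the ObjectType data-table row into GridChildren.
; Straight steps become instanced meshes and corners separate static meshes, with collision boxes added along the path.
; Border pieces sit offset half a cell to the side and get extra boxes at corners.
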(event EventBeginPlay)

(event Collision|EventActorBeginOverlap
  (params (OtherActor :type Actor%20Object%20Reference)))

(event EventTick
  (params (DeltaSeconds :type Float%20%28single-precision%29)))

(fn ConstructionScript
  (CallFunction|BuildArray))

(fn BuildArray
  (bind _gridchildren (Variables|Default|GetGridChildren))
  (Utilities|Array|Clear (Variables|Default|GetGridChildren))
  (bind _returnvalue (Utilities|GetDataTableRow "/Game/Blueprints/Buildings/BuldingData.BuldingData" (Variables|Default|GetObjectType))
    (:then
      (Components|StaticMesh|SetStaticMesh (Variables|Default|GetInstancedStaticMesh) (Utilities|Array|Get(acopy) (.Mesh (Utilities|Struct|BreakBuildingInfo _returnvalue))))
      (for _array_element (Variables|Default|GetDirs)
        (LocalVariables|SetDir _array_element)
        (LocalVariables|SetPrevRotation (LocalVariables|GetRotation))
        (bind _output_get (LocalVariables|SetPrev (LocalVariables|GetCurrent)))
        (LocalVariables|SetCurrentPos (CallFunction|GetGridPos _output_get (LocalVariables|GetCurrentPos)))
        (bind _output_get_2 (LocalVariables|SetCurrent (Utilities|Enum|ByteToEnumEDirection (Class|KismetMathLibrary|PercentByteByte (+ (Utilities|Select :Index (LocalVariables|GetDir) :NewEnumerator0 0 :NewEnumerator1 1 :NewEnumerator2 3 :NewEnumerator3 0) (LocalVariables|GetCurrent)) 4))))
        (LocalVariables|SetRotation (CallFunction|GetRotation _output_get_2))
        (bind _output_get_3 (LocalVariables|SetNewLocalVar_0 (CallFunction|RoundVector (Math|Vector|RotateVector (CallFunction|IntVectortoVector (LocalVariables|GetNewLocalVar_0)) (Math|Rotator|MakeRotator 0.0 0.0 (Utilities|Select :Index (LocalVariables|GetDir) :NewEnumerator0 0.0 :NewEnumerator1 9e+01 :NewEnumerator2 -9e+01 :NewEnumerator3 0.0))))))
        (bind _returnvalue_2 (Utilities|Array|Add _gridchildren (Utilities|Struct|MakeGridTransform (LocalVariables|GetCurrentPos) _output_get_3 (.walkabletiles (Utilities|Struct|BreakBuildingInfo _returnvalue)) (.block (Utilities|Struct|BreakBuildingInfo _returnvalue)) (.blockPercentage (Utilities|Struct|BreakBuildingInfo _returnvalue)) (.border (Utilities|Struct|BreakBuildingInfo _returnvalue)) (.isUpToEdge (Utilities|Struct|BreakBuildingInfo _returnvalue)) (.isCorner (Utilities|Struct|BreakBuildingInfo _returnvalue)))))
        (switch Utilities|FlowControl|Switch|SwitchonDir (LocalVariables|GetDir)
          (:NewEnumerator0
            _)
          (:NewEnumerator1
            (Utilities|Array|Add (Variables|Default|GetGridChildren) (Utilities|Struct|MakeGridTransform (LocalVariables|GetCurrentPos) (.Direction (Utilities|Struct|BreakGridTransform (Utilities|Array|Get(acopy) _gridchildren (- _returnvalue_2 1)))) (.walkabletiles (Utilities|Struct|BreakBuildingInfo _returnvalue)) (.block (Utilities|Struct|BreakBuildingInfo _returnvalue)) (.blockPercentage (Utilities|Struct|BreakBuildingInfo _returnvalue)) (.border (Utilities|Struct|BreakBuildingInfo _returnvalue)) (.isUpToEdge (Utilities|Struct|BreakBuildingInfo _returnvalue)) (.isCorner (Utilities|Struct|BreakBuildingInfo _returnvalue))) :!label _label))
          (:NewEnumerator2
            (goto _label))
          (:NewEnumerator3
            _))
        (switch Utilities|FlowControl|Switch|SwitchonDir (LocalVariables|GetDir)
          (:NewEnumerator0
            (Components|InstancedStaticMesh|AddInstance (Variables|Default|GetInstancedStaticMesh) (Math|Transform|MakeTransform (CallFunction|GetPostion (.border (Utilities|Struct|BreakBuildingInfo _returnvalue)) (LocalVariables|GetCurrentPos) (LocalVariables|GetPrev)) (Math|Rotator|MakeRotator 0.0 0.0 (LocalVariables|GetPrevRotation)) "1,1,1"))
            (CallFunction|AddCollisionBox (CallFunction|GetPostion (.border (Utilities|Struct|BreakBuildingInfo _returnvalue)) (LocalVariables|GetCurrentPos) (LocalVariables|GetPrev)) (.BoxCollision (Utilities|Struct|BreakBuildingInfo _returnvalue)) (LocalVariables|GetPrevRotation) :!label _label_2))
          (:NewEnumerator1
            (bind _returnvalue_3 (AddComponent|AddStaticMeshComponent false (Math|Transform|MakeTransform (CallFunction|GetPostion (.border (Utilities|Struct|BreakBuildingInfo _returnvalue)) (LocalVariables|GetCurrentPos) (LocalVariables|GetPrev)) (Math|Rotator|MakeRotator 0.0 0.0 (LocalVariables|GetPrevRotation)) "1,1,1")))
            (Components|StaticMesh|SetStaticMesh _returnvalue_3 (.ClockWise (Utilities|Struct|BreakBuildingInfo _returnvalue)))
            (if (.border (Utilities|Struct|BreakBuildingInfo _returnvalue))
              (CallFunction|AddCollisionBox (CallFunction|GetPostion true (LocalVariables|GetCurrentPos) (LocalVariables|GetCurrent)) (.BoxCollision (Utilities|Struct|BreakBuildingInfo _returnvalue)) (LocalVariables|GetRotation))
              (goto _label_2)
              (else
                (goto _label_2))))
          (:NewEnumerator2
            (bind _returnvalue_4 (AddComponent|AddStaticMeshComponent false (Math|Transform|MakeTransform (CallFunction|GetPostion (.border (Utilities|Struct|BreakBuildingInfo _returnvalue)) (LocalVariables|GetCurrentPos) (LocalVariables|GetPrev)) (Math|Rotator|MakeRotator 0.0 0.0 (LocalVariables|GetPrevRotation)) "1,1,1")))
            (Components|StaticMesh|SetStaticMesh _returnvalue_4 (.AntiClockWise (Utilities|Struct|BreakBuildingInfo _returnvalue)))
            (Utilities|FlowControl|Sequence
              (:then_0
                (goto _label_2))
              (:then_1
                (if (.border (Utilities|Struct|BreakBuildingInfo _returnvalue))
                  (bind _b (CallFunction|AddBord (LocalVariables|GetCurrent)))
                  (LocalVariables|SetCurrentPos (CallFunction|AddIntVector _b (LocalVariables|GetCurrentPos)))
                  (CallFunction|AddCollisionBox (CallFunction|GetPostion true (LocalVariables|GetCurrentPos) (LocalVariables|GetCurrent)) (.BoxCollision (Utilities|Struct|BreakBuildingInfo _returnvalue)) (LocalVariables|GetRotation)))))))))))

(fn GetRotation
  (params (Index :type EDirection%20Enum :default "D_Forward"))
  (return (Utilities|Select :Index Index :D_Forward 0.0 :D_Rightward 9e+01 :D_Backward 1.8e+02 :D_Leftward 2.7e+02 :D_Upward 0.0 :D_Downward 0.0)))

(fn GetGridPos
  (params (DirectionFacing :type EDirection%20Enum :default "D_Forward") (CurrentPos :type Int%20Vector%20Structure))
  (return (CallFunction|AddIntVector (CallFunction|RoundVector (Math|Vector|RotateVectorAroundAxis "1.000000, 0, 0" (CallFunction|GetRotation DirectionFacing) "0.000000, 0,1.000000")) CurrentPos)))

(fn GetPostion
  (params (InputPin :type Boolean) (InIntVector :type Int%20Vector%20Structure%20%28by%20ref%29) (Index :type EDirection%20Enum :default "D_Forward"))
  (return (+ (* (Math|Conversions|ToVector(Float) InIntVector) 1e+02) (select InputPin (Math|Vector|RotateVectorAroundAxis "0.000000,-50.000000, 0" (CallFunction|GetRotation Index) "0, 0,1.000000") "0, 0, 0"))))

(fn PrintonDebug
  (params (InString :type String))
  (if (Variables|Default|GetDebug)
    (Development|PrintString InString true true "(R=0.000000,G=0.660000,B=1.000000,A=1.000000)" 1e+01)))

(fn AddCollisionBox
  (params (Location :type Vector) (BoxExtent :type Vector) (Relative%20Transform%20Rotation%20Z%20%28Yaw%29 :type Float%20%28single-precision%29))
  (bind _returnvalue (AddComponent|AddBoxComponent false (Math|Transform|MakeTransform (+ Location (Math|Vector|MakeVector 0.0 0.0 (.Z (Math|Vector|BreakVector BoxExtent)))) (Math|Rotator|MakeRotator 0.0 0.0 Relative%20Transform%20Rotation%20Z%20%28Yaw%29) "1,1,1")))
  (Components|Box|SetBoxExtent _returnvalue BoxExtent true))

(fn AddBord
  (params (Index :type EDirection%20Enum :default "D_Forward"))
  (return (CallFunction|RoundVector (Math|Vector|RotateVectorAroundAxis "1.000000,1.000000, 0" (CallFunction|GetRotation Index) "0.000000, 0,1.000000"))))