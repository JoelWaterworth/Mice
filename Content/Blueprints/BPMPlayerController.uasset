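; Player controller for a grid-based unit game, handling the hover cursor, unit selection and move orders.
; On Remote it spawns the cursor and HUD widget, then snaps the cursor to the traced WorldGrid cell each tick.
; Select calculates range-limited paths for a same-team unit.
; Target turns those into a route for CreateWalkCommand, which queues a WalkCommand only on authority; a separate event recolours the HUD by team.
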(event Custom|CreateWalkCommand
  (params (NewParam2 :type BP%20Unit%20Object%20Reference) (path :type Array%20of%20Int%20Vector%20Structures))
  (Networking|SwitchHasAuthority
    (:Authority
      (bind _returnvalue (Game|ConstructObjectfromClass "/Game/Blueprints/WalkCommand.WalkCommand_C" self))
      (Variables|/Game/Blueprints/WalkCommand.WalkCommand_C|Setunit _returnvalue NewParam2)
      (Variables|/Game/Blueprints/WalkCommand.WalkCommand_C|Setpath _returnvalue path)
      (Utilities|Array|Add (Variables|Default|Getcommands) _returnvalue))))

(event EventBeginPlay
  (Networking|SwitchHasAuthority
    (:Remote
      (bind _outactors (Actor|GetAllActorsOfClass "/Script/Mice.WorldGrid"))
      (bind _returnvalue (Game|SpawnActorfromClass "/Game/Blueprints/cursor.cursor_C" (Class|WorldGrid|VectortoWorldTransform (Utilities|Array|Get(acopy) _outactors)) "AlwaysSpawn" 0 0))
      (Variables|Default|Setcursor _returnvalue)
      (bind _returnvalue_2 (UserInterface|CreateWidget "/Game/Blueprints/BPWidget.BPWidget_C" self))
      (Variables|Default|SetGUI _returnvalue_2)
      (UserInterface|Viewport|AddtoViewport _returnvalue_2 0))))

(event EventTick
  (params (DeltaSeconds :type Float%20%28single-precision%29))
  (bind (_hitresult _returnvalue) (Game|Player|GetHitResultUnderCursorbyChannel "TraceTypeQuery3" true))
  (bind _cursor (Variables|Default|Getcursor))
  (bind (_bblockinghit _binitialoverlap _time _distance _location _impactpoint _normal _impactnormal _physmat _hitactor _hitcomponent) (Collision|BreakHitResult _hitresult))
  (Networking|SwitchHasAuthority
    (:Remote
      (if _returnvalue
        (bind _asgrid_collision (Utilities|Casting|CastToGridCollision _hitcomponent))
        (bind _asworld_grid (Utilities|Casting|CastToWorldGrid _hitactor))
        (Utilities|IsValid _cursor
          (:Is%20Valid
            (Transformation|SetActorTransform _cursor (Class|WorldGrid|VectortoWorldTransform _asworld_grid (Variables|/Script/Mice.GridCollision|Getpos _asgrid_collision)))))))))

(event EventUpdatePlayerTeam
  (params (team :type ETeam%20Enum :default "T_Blue"))
  (bind _gui (Variables|Default|GetGUI))
  (Utilities|IsValid _gui
    (:Is%20Valid
      (Default|UpdateColours _gui team))))

(event Input|ActionEvents|InputActionSelect
  (params (Key :type Key%20Structure))
  (bind (_hitresult _returnvalue) (Game|Player|GetHitResultUnderCursorbyChannel "TraceTypeQuery3" true))
  (:Pressed
    (if _returnvalue
      (bind _asbpunit (Utilities|Casting|CastToBPUnit (.HitActor (Collision|BreakHitResult _hitresult))))
      (bind _asmplayer_state (Utilities|Casting|CastToMPlayerState (Variables|Default|GetPlayerState)))
      (if (Utilities|Enum|Equal(Enum) (Variables|/Script/Mice.Unit|Getteam _asbpunit) (Variables|/Script/Mice.MPlayerState|Getteam _asmplayer_state))
        (bind _outactors (Actor|GetAllActorsOfClass "/Game/Blueprints/BPWorldGrid.BPWorldGrid_C"))
        (bind _returnvalue_2 (Class|WorldGrid|CalculatePaths (Utilities|Array|Get(acopy) _outactors) _asbpunit 8))
        (Variables|Default|SetPaths _returnvalue_2)
        (Variables|Default|Setselected _asbpunit)
        (Rendering|SetVisibility (Variables|/Script/Mice.Unit|GetselectPlane _asbpunit) true false)))))

(event Input|ActionEvents|InputActionTarget
  (params (Key :type Key%20Structure))
  (bind (_hitresult _returnvalue) (Game|Player|GetHitResultUnderCursorbyChannel "TraceTypeQuery3" true))
  (:Pressed
    (if _returnvalue
      (bind _asgrid_collision (Utilities|Casting|CastToGridCollision (.HitComponent (Collision|BreakHitResult _hitresult))))
      (CallFunction|CreateWalkCommand (Variables|Default|Getselected) (Class|WorldGrid|CreatePathfromRoutes (Variables|Default|GetPaths) (Variables|/Script/Mice.GridCollision|Getpos _asgrid_collision))))))

(fn ConstructionScript)