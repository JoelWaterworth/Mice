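; Player controller for a grid-based unit game that handles cursor display, unit selection and move orders.
; On the remote side it creates the GUI and a cursor actor, which Tick snaps to the WorldGrid cell under the mouse.
; Select highlights the clicked unit and caches range-limited paths from the grid.
; Target builds a route to the clicked cell and passes it to CreateWalkCommand, which queues a WalkCommand only on authority.
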(event Custom|createWalkCommand
  (params (NewParam2 :type BP%20Unit%20Object%20Reference) (NewParam :type Array%20of%20Vector%202D%20Int%20Structures))
  (Networking|SwitchHasAuthority
    (:Authority
      (bind _returnvalue (Game|ConstructObjectfromClass "/Game/Blueprints/walkCommand.walkCommand_C" self))
      (Variables|/Game/Blueprints/walkCommand.walkCommand_C|Setunit _returnvalue NewParam2)
      (Variables|/Game/Blueprints/walkCommand.walkCommand_C|Setpath _returnvalue NewParam)
      (Utilities|Array|Add (Variables|Default|Getcommands) _returnvalue))))

(event EventBeginPlay
  (Networking|SwitchHasAuthority
    (:Remote
      (bind _outactors (Actor|GetAllActorsOfClass "/Script/Mice.WorldGrid"))
      (bind _returnvalue (Game|SpawnActorfromClass (Variables|Default|GetNewVar_0) (Class|WorldGrid|VectortoWorldTransform (Utilities|Array|Get(acopy) _outactors)) "Undefined" 0 0))
      (Variables|Default|Setcursor _returnvalue)
      (bind _returnvalue_2 (UserInterface|CreateWidget "/Game/Blueprints/BPGUI.BPGUI_C" self))
      (UserInterface|Viewport|AddtoViewport _returnvalue_2 0))))

(event EventTick
  (params (DeltaSeconds :type Float%20%28single-precision%29))
  (bind (_hitresult _returnvalue) (Game|Player|GetHitResultUnderCursorbyChannel "TraceTypeQuery3" true))
  (bind (_bblockinghit _binitialoverlap _time _distance _location _impactpoint _normal _impactnormal _physmat _hitactor _hitcomponent) (Collision|BreakHitResult _hitresult))
  (Networking|SwitchHasAuthority
    (:Remote
      (if _returnvalue
        (bind _asgrid_collision (Utilities|Casting|CastToGridCollision _hitcomponent))
        (bind _asworld_grid (Utilities|Casting|CastToWorldGrid _hitactor))
        (Transformation|SetActorTransform (Variables|Default|Getcursor) (Class|WorldGrid|VectortoWorldTransform _asworld_grid (Variables|/Script/Mice.GridCollision|Getpos _asgrid_collision)))))))

(event Input|ActionEvents|InputActionSelect
  (params (Key :type Key%20Structure))
  (bind (_hitresult _returnvalue) (Game|Player|GetHitResultUnderCursorbyChannel "TraceTypeQuery3" true))
  (:Pressed
    (if _returnvalue
      (bind _asbpunit (Utilities|Casting|CastToBPUnit (.HitActor (Collision|BreakHitResult _hitresult))))
      (bind _outactors (Actor|GetAllActorsOfClass "/Game/Blueprints/BPWorldGrid.BPWorldGrid_C"))
      (bind _returnvalue_2 (Class|WorldGrid|CalculatePaths (Utilities|Array|Get(acopy) _outactors) _asbpunit 8))
      (Variables|Default|Setpaths _returnvalue_2)
      (Variables|Default|SetNewVar_1 _asbpunit)
      (Rendering|SetVisibility (Variables|/Script/Mice.Unit|GetselectPlane _asbpunit) true false))))

(event Input|ActionEvents|InputActionTarget
  (params (Key :type Key%20Structure))
  (bind (_hitresult _returnvalue) (Game|Player|GetHitResultUnderCursorbyChannel "TraceTypeQuery3" true))
  (:Pressed
    (if _returnvalue
      (bind _asgrid_collision (Utilities|Casting|CastToGridCollision (.HitComponent (Collision|BreakHitResult _hitresult))))
      (CallFunction|CreateWalkCommand (Variables|Default|GetNewVar_1) (Class|WorldGrid|CreatePathfromRoutes (Variables|Default|Getpaths) (Variables|/Script/Mice.GridCollision|Getpos _asgrid_collision))))))

(fn ConstructionScript)