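; Player controller for mouse-driven unit selection and movement on a world grid.
; Left-clicking a BPUnit shows its Plane, stores it as Target and caches paths calculated by the first BPWorldGrid within Limit.
; Clicking a GridCollision component with a Target set rebuilds the route from that cached came-from data and passes it to MoveTo.
; Tick snaps a cursor actor, spawned at BeginPlay, to the hovered tile.
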(event EventBeginPlay
  (Variables|Default|SetbShowMouseCursor true)
  (bind _returnvalue (Game|SpawnActorfromClass "/Game/Blueprints/BPTileCursor.BPTileCursor_C" (Math|Transform|MakeTransform "0, 0, 0") "Undefined" 0 0))
  (Variables|Default|SetTile%20Cursor _returnvalue))

(event EventTick
  (params (DeltaSeconds :type Float%20%28single-precision%29))
  (bind _hitresult (Game|Player|GetHitResultUnderCursorbyChannel "TraceTypeQuery3" true))
  (bind (_bblockinghit _binitialoverlap _time _distance _location _impactpoint _normal _impactnormal _physmat _hitactor _hitcomponent) (Collision|BreakHitResult _hitresult))
  (bind _asgrid_collision (Utilities|Casting|CastToGridCollision _hitcomponent))
  (bind _asbpworld_grid (Utilities|Casting|CastToBPWorldGrid _hitactor))
  (Transformation|SetActorTransform (Variables|Default|GetTile%20Cursor) (Default|Vector2DInttoWorldTransform _asbpworld_grid (Variables|/Script/Mice.GridCollision|Getpos _asgrid_collision))))

(event Input|MouseEvents|LeftMouseButton
  (params (Key :type Key%20Structure))
  (bind _hitresult (Game|Player|GetHitResultUnderCursorbyChannel "TraceTypeQuery3" true))
  (bind (_bblockinghit _binitialoverlap _time _distance _location _impactpoint _normal _impactnormal _physmat _hitactor _hitcomponent) (Collision|BreakHitResult _hitresult))
  (:Pressed
    (bind _asbpunit (Utilities|Casting|CastToBPUnit _hitactor)
      (:then
        (Rendering|SetVisibility (Variables|/Game/Blueprints/BPUnit.BPUnit_C|GetPlane _asbpunit) true false)
        (bind _output_get (Variables|Default|SetTarget _asbpunit))
        (bind _outactors (Actor|GetAllActorsOfClass "/Game/Blueprints/BPWorldGrid.BPWorldGrid_C"))
        (bind _camefrom1 (Default|CalculatePaths (Utilities|Array|Get(acopy) _outactors) _output_get (Variables|Default|GetLimit)))
        (Variables|Default|SetPath _camefrom1))
      (:CastFailed
        (Utilities|IsValid (Variables|Default|GetTarget)
          (:Is%20Valid
            (bind _asgrid_collision (Utilities|Casting|CastToGridCollision _hitcomponent)
              (:then
                (Default|Moveto (Variables|Default|GetTarget) (CallFunction|CamefromtoPath (Variables|/Script/Mice.GridCollision|Getpos _asgrid_collision) (Variables|Default|GetPath))))
              (:CastFailed
                (Development|PrintString (Utilities|GetDisplayName _hitcomponent)))))
          (:Is%20Not%20Valid
            (Development|PrintString "No target")))))))

(fn ConstructionScript)