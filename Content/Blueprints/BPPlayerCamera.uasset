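; BPPlayerCamera is a player camera Blueprint that pans through the world from Forward and Rightward axis input.
; Each axis value is scaled by a shared speed variable (NewVar0) and rotated 45 degrees about world Z, aligning movement to a diagonal heading.
; The result is applied as a world transform offset on every axis event, with no delta time scaling.
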(event Input|AxisEvents|InputAxisForward
  (params (AxisValue :type Float%20%28single-precision%29))
  (Class|Actor|AddActorWorldTransform (Math|Transform|MakeTransform (Math|Vector|RotateVectorAroundAxis (Math|Vector|MakeVector (* AxisValue (Variables|Default|GetNewVar_0)) 0.0 0.0) -45.0 "0, 0,1.000000") "0, 0, 0" "1,1,1") false false))

(event Input|AxisEvents|InputAxisRightward
  (params (AxisValue :type Float%20%28single-precision%29))
  (Class|Actor|AddActorWorldTransform (Math|Transform|MakeTransform (Math|Vector|RotateVectorAroundAxis (Math|Vector|MakeVector 0.0 (* AxisValue (Variables|Default|GetNewVar_0)) 0.0) -45.0 "0, 0,1.000000") "0, 0, 0" "1,1,1") false false))

(fn ConstructionScript)