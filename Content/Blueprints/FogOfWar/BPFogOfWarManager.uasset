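; Fog of war manager that displays the fog through a post-process dynamic material created in the construction script.
; Texture updates pass the current and previous fog textures to the material and reset Blend to zero.
; Tick has logic to ramp Blend toward one for a crossfade, but only while it is below zero, so otherwise it just sets IsDoneBlending.
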(event EventTick
  (params (DeltaSeconds :type Float%20%28single-precision%29))
  (bind _self self)
  (if (< (Variables|Default|GetFOWTexture%20Blend) 0.0)
    (bind _output_get (Variables|Default|SetFOWTexture%20Blend (Math|Float|Clamp(Float) (+ (* DeltaSeconds 1e+01) (Variables|Default|GetFOWTexture%20Blend)))))
    (Rendering|Material|SetScalarParameterValue (Variables|Default|GetDynamic%20Mat) "Blend" _output_get :!class /Script/Engine.MaterialInstanceDynamic)
    (elif (not (Variables|Default|GetbIsDoneBlending _self))
      (Variables|Default|SetbIsDoneBlending _self true))))

(event EventOnFowTextureUpdated
  (params (currentTexture :type Texture%202D%20Object%20Reference) (lastTexture :type Texture%202D%20Object%20Reference))
  (bind _dynamic_mat (Variables|Default|GetDynamic%20Mat))
  (Rendering|Material|SetTextureParameterValue _dynamic_mat "FoWTexture" currentTexture)
  (Rendering|Material|SetTextureParameterValue _dynamic_mat "LastFOWTexture" lastTexture)
  (Rendering|Material|SetScalarParameterValue _dynamic_mat "Blend" 0.0 :!class /Script/Engine.MaterialInstanceDynamic)
  (Variables|Default|SetFOWTexture%20Blend 0.0))

(fn ConstructionScript
  (bind _returnvalue (Rendering|Material|CreateDynamicMaterialInstance 0 :!class /Script/Engine.KismetMaterialLibrary))
  (Variables|Default|SetDynamic%20Mat _returnvalue)
  (Rendering|AddorUpdateBlendable (Variables|Default|GetPostProcess) _returnvalue 1.0 :!class /Script/Engine.PostProcessComponent))