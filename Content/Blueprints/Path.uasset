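; Actor that draws a unit's movement path as a visible ribbon of spline meshes.
; On BeginPlay it builds a spline from its own origin through the Path points, scaled by 100 and raised by PathHeight.
; It then lays a spline mesh segment every 100 units along the length, using the configured mesh and material.
; It binds to its owning BPUnit's finish-path event and destroys itself when that fires.
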(event Custom|Path%20Finished
  (Actor|DestroyActor))

(event EventBeginPlay
  (bind _spline (Variables|Default|GetSpline))
  (bind _spline_2 (Variables|Default|GetSpline))
  (bind _path (Variables|Default|GetPath))
  (Utilities|FlowControl|Sequence
    (:then_0
      (Spline|SetLocationatSplinePoint (Variables|Default|GetSpline) 0 (Math|Vector|MakeVector 0.0 0.0 (Variables|Default|Getpath%20height)) "Local" true)
      (for _index (range 1 (Utilities|Array|Length _path))
        (Class|SplineComponent|AddPoint (Variables|Default|GetSpline) (Utilities|Struct|MakeSplinePoint (Math|Conversions|ToFloat(Integer) _index) (+ (* (Math|Conversions|ToVector(Float) (Utilities|Array|Get(acopy) _path (- _index 1))) 1e+02) (Math|Vector|MakeVector 0.0 0.0 (Variables|Default|Getpath%20height)))) false))
      (Spline|UpdateSpline (Variables|Default|GetSpline)))
    (:then_1
      (for _index_2 (range 0 (Math|Float|Floor (/ (Spline|GetSplineLength (Variables|Default|GetSpline)) 1e+02)))
        (bind _returnvalue (AddComponent|AddSplineMeshComponent true (Transformation|GetActorTransform)))
        (Components|StaticMesh|SetStaticMesh _returnvalue (Variables|Default|Getmesh))
        (Rendering|Material|SetMaterial _returnvalue 0 (Variables|Default|GetMaterial%20Instance))
        (SplineMesh|SetStartandEnd _returnvalue (Spline|GetLocationatDistanceAlongSpline _spline (Math|Conversions|ToFloat(Integer) (* _index_2 100)) "Local") (Spline|GetTangentatDistanceAlongSpline _spline (Math|Conversions|ToFloat(Integer) (* _index_2 100)) "Local") (Spline|GetLocationatDistanceAlongSpline _spline_2 (+ (Math|Conversions|ToFloat(Integer) (* _index_2 100)) 1e+02) "Local") (Spline|GetTangentatDistanceAlongSpline _spline_2 (+ (Math|Conversions|ToFloat(Integer) (* _index_2 100)) 1e+02) "Local") true :!class /Script/Engine.SplineMeshComponent)))
    (:then_2
      (bind _asbpunit (Utilities|Casting|CastToBPUnit (Components|GetOwner))
        (:then
          (EventDispatchers|BindEventtoFinishPath _asbpunit (delegate Custom|Path%20Finished)))
        (:CastFailed
          (Development|PrintString "Cast failed"))))))

(fn ConstructionScript)