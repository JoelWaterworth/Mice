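; Utility functions for integer vector math and conversion between float and integer vectors.
; Provides component-wise equality, addition and subtraction, plus conversion to integers by flooring each axis and back to floats.
; Centre shifts a position by a fixed half-step of 50 units in X and Y, leaving Z unchanged, which suggests centring on 100-unit grid cells.
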(fn Eq
  (params (A :type Int%20Vector%20Structure) (B :type Int%20Vector%20Structure))
  (return (Math|Boolean|ANDBoolean (== (.x A) (.x B)) (== (.y A) (.y B)) (== (.z A) (.z B)))))

(fn VectortoIntVector
  (params (NewParam :type Vector))
  (return (Utilities|Struct|MakeIntVector (Math|Float|Floor (.x NewParam)) (Math|Float|Floor (.y NewParam)) (Math|Float|Floor (.z NewParam)))))

(fn Centre
  (params (NewParam :type Vector))
  (return (+ NewParam "50.000000,50.000000, 0")))

(fn IntVectortoVector
  (params (in :type Int%20Vector%20Structure))
  (return (Math|Vector|MakeVector (Math|Conversions|ToFloat(Integer) (.x in)) (Math|Conversions|ToFloat(Integer) (.y in)) (Math|Conversions|ToFloat(Integer) (.z in)))))

(fn AddIntVector
  (params (A :type Int%20Vector%20Structure) (B :type Int%20Vector%20Structure))
  (return (Utilities|Struct|MakeIntVector (+ (.x A) (.x B)) (+ (.y A) (.y B)) (+ (.z A) (.z B)))))

(fn SubIntVector
  (params (A :type Int%20Vector%20Structure) (B :type Int%20Vector%20Structure))
  (return (Utilities|Struct|MakeIntVector (- (.x A) (.x B)) (- (.y A) (.y B)) (- (.z A) (.z B)))))