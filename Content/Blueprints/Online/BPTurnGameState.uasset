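; Game state for an online two-team, turn-based unit game, handling turn order and the win condition.
; Submitted commands from a player controller run only on that team's turn, then get cleared as the turn flips between Blue and Red.
; At begin play it counts each team's BPUnit actors and binds their destruction, calling game over with the opposing team when either count reaches zero.
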(event Custom|On%20unit%20destroy
  (params (DestroyedActor :type Actor%20Object%20Reference))
  (bind _asbpunit (Utilities|Casting|CastToBPUnit DestroyedActor))
  (bind _result (Math|Integer|DecrementInt (Utilities|Select :Index (Variables|/Script/Mice.Unit|Getteam _asbpunit) :T_Blue (Variables|Default|GetNumberOfBlueUnits) :T_Red (Variables|Default|GetNumberOfRedUnits)))
    (:%20%20
      (if (<= _result 0)
        (Default|CallGameOver (Utilities|Select :Index (Variables|/Script/Mice.Unit|Getteam _asbpunit) :T_Blue "T_Red" :T_Red "T_Blue"))))))

(event EventBeginPlay
  (bind _outactors (Actor|GetAllActorsOfClass "/Game/Blueprints/Player/BPUnit.BPUnit_C"))
  (for _array_element _outactors
    (Game|AssignOnDestroyed _array_element (delegate Custom|On%20unit%20destroy))
    (Math|Integer|IncrementInt (Utilities|Select :Index (Variables|/Script/Mice.Unit|Getteam _array_element) :T_Blue (Variables|Default|GetNumberOfBlueUnits) :T_Red (Variables|Default|GetNumberOfRedUnits)))))

(event EventSumbitCommands
  (params (playerController :type M%20Player%20Controller%20Object%20Reference))
  (bind _asmplayer_state (Utilities|Casting|CastToMPlayerState (Variables|/Script/Engine.Controller|GetPlayerState playerController)))
  (if (Math|Boolean|Equal(Boolean) (Variables|Default|GetIsBluesTurn) (Utilities|Select :Index (Variables|/Script/Mice.MPlayerState|Getteam _asmplayer_state) :T_Blue true :T_Red false))
    (Class|MGameState|ExecuteCommands (Class|MPlayerController|GetCommands playerController))
    (Class|MPlayerController|ClearCommands playerController)
    (Variables|Default|SetIsBluesTurn (not (Variables|Default|GetIsBluesTurn)))
    (else
      (Development|PrintString "Not your turn"))))

(fn ConstructionScript)