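; Capture-zone objective for a turn-based game that ends the match when one team holds it for enough turns.
; The construction script snaps the box to the 100-unit grid and builds a procedural mesh quad matching its footprint.
; Overlap and unit-destroyed events rebuild the list of teams inside.
; On authority, each turn end counts down for a sole team, resets when contested or switching teams, and calls game over at zero.
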(event OnComponentBeginOverlap(Box)
  (params (OverlappedComponent :type Primitive%20Component%20Object%20Reference) (OtherActor :type Actor%20Object%20Reference) (OtherComp :type Primitive%20Component%20Object%20Reference) (OtherBodyIndex :type Integer) (bFromSweep :type Boolean) (SweepResult :type Hit%20Result%20Structure%20%28by%20ref%29))
  (bind _asbpunit (Utilities|Casting|CastToBPUnit OtherActor))
  (if (CallFunction|BoundryCheck (Variables|/Script/Mice.Unit|Getpos _asbpunit))
    (CallFunction|Update)))

(event OnComponentEndOverlap(Box)
  (params (OverlappedComponent :type Primitive%20Component%20Object%20Reference) (OtherActor :type Actor%20Object%20Reference) (OtherComp :type Primitive%20Component%20Object%20Reference) (OtherBodyIndex :type Integer))
  (bind _asbpunit (Utilities|Casting|CastToBPUnit OtherActor))
  (Game|UnbindEventfromOnDestroyed _asbpunit (delegate Custom|Overlapping%20Actor%20Destroyed))
  (CallFunction|Update))

(event Custom|Overlapping%20Actor%20Destroyed
  (params (DestroyedActor :type Actor%20Object%20Reference))
  (CallFunction|Update))

(event Custom|Turn%20Over
  (CallFunction|UpdateCapture)
  (if (== (Variables|Default|GetTurnsLeft) 0)
    (bind _asbpturn_game_state (Utilities|Casting|CastToBPTurnGameState (Game|GetGameState)))
    (Default|CallGameOver _asbpturn_game_state (Variables|Default|GetPrevousTeam))))

(event Custom|Update
  (CallFunction|UpdateOverlappingActor (delegate Custom|Overlapping%20Actor%20Destroyed)))

(event EventBeginPlay
  (Networking|SwitchHasAuthority
    (:Authority
      (bind _asbpturn_game_state (Utilities|Casting|CastToBPTurnGameState (Game|GetGameState)))
      (EventDispatchers|BindEventtoTurnOver _asbpturn_game_state (delegate Custom|Turn%20Over)))))

(fn ConstructionScript
  (bind _box (Variables|Default|GetBox))
  (bind _newlocalvar_0 (LocalVariables|GetNewLocalVar_0))
  (bind _proceduralmesh (Variables|Default|GetProceduralMesh))
  (bind _output_get (Variables|Default|SetBoxExtent (- (* (Math|Conversions|ToVector(Float) (CallFunction|RoundVector (/ (Variables|Default|GetBoxExtent) 1e+02))) 1e+02) "50.000000,50.000000,50.000000")))
  (Components|Box|SetBoxExtent _box _output_get true)
  (Transformation|SetRelativeLocation _box (Math|Vector|MakeVector 0.0 0.0 (.Z (Math|Vector|BreakVector _output_get))) false false)
  (Utilities|FlowControl|Sequence
    (:then_0
      (Utilities|Array|SetArrayElem _newlocalvar_0 0 (Math|Vector|MakeVector (* (.x (Variables|Default|GetBoxExtent)) -1.0) (.y (Variables|Default|GetBoxExtent)) 0.0)))
    (:then_1
      (Utilities|Array|SetArrayElem _newlocalvar_0 1 (Math|Vector|MakeVector (.x (Variables|Default|GetBoxExtent)) (.y (Variables|Default|GetBoxExtent)) 0.0)))
    (:then_2
      (Utilities|Array|SetArrayElem _newlocalvar_0 2 (Math|Vector|MakeVector (* (.x (Variables|Default|GetBoxExtent)) -1.0) (* (.y (Variables|Default|GetBoxExtent)) -1.0) 0.0)))
    (:then_3
      (Utilities|Array|SetArrayElem _newlocalvar_0 3 (Math|Vector|MakeVector (.x (Variables|Default|GetBoxExtent)) (* (.y (Variables|Default|GetBoxExtent)) -1.0) 0.0)))
    (:then_4
      (Class|ProceduralMeshComponent|CreateMeshSectionLinearColor _proceduralmesh 0 (LocalVariables|GetNewLocalVar_0) (Utilities|Array|MakeArray 0 1 2 3 2 1) 0 (Utilities|Array|MakeArray "(X=-1.000000,Y=1.000000)" "(X=1.000000,Y=1.000000)" "(X=-1.000000,Y=-1.000000)" "(X=1.000000,Y=0.000000)") 0 0 false)
      (Rendering|Material|SetMaterial _proceduralmesh 0 (Variables|Default|GetNaterial)))))

(fn BoundryCheck
  (params (location :type Int%20Vector%20Structure))
  (bind _gridorigin (Variables|Default|GetGridOrigin))
  (bind _boxextent (Variables|Default|GetBoxExtent))
  (bind _returnvalue (/ _boxextent 1e+02))
  (bind _b (CallFunction|RoundVector _returnvalue))
  (bind _c (CallFunction|AddIntVector (.origin _gridorigin) _b))
  (bind _c_2 (CallFunction|SubIntVector (.origin _gridorigin) _b))
  (return (not (or (Math|Boolean|ANDBoolean (> (.x location) (.x _c)) (> (.y location) (.y _c)) (> (.z location) (.z _c))) (Math|Boolean|ANDBoolean (< (.x location) (.x _c_2)) (< (.y location) (.y _c_2)) (< (.z location) (.z _c_2)))))))

(fn UpdateOverlappingActor
  (params (Event :type Delegate%20%28by%20ref%29))
  (Utilities|Array|Clear (Variables|Default|GetCapturingTeams))
  (for _array_element (Collision|GetOverlappingActors (Variables|Default|GetBox) "/Game/Blueprints/Player/BPUnit.BPUnit_C" :!class /Script/Engine.PrimitiveComponent)
    (bind _asbpunit (Utilities|Casting|CastToBPUnit _array_element))
    (Game|BindEventtoOnDestroyed _array_element Event)
    (Utilities|Array|Add (Variables|Default|GetCapturingTeams) (Variables|/Script/Mice.Unit|Getteam _asbpunit)))
  (return (Variables|Default|GetCapturingTeams)))

(fn UpdateCapture
  (bind _capturingteams (Variables|Default|GetCapturingTeams))
  (if (> (Utilities|Array|Length _capturingteams) 0)
    (LocalVariables|SetfirstUnit (Utilities|Array|Get(acopy) _capturingteams))
    (bind _array_element (Utilities|Array|ForEachLoopwithBreak _capturingteams)
      (:LoopBody
        (if (not (Utilities|Enum|Equal(Enum) _array_element (LocalVariables|GetfirstUnit)))
          (Variables|Default|SetTurnsLeft (Variables|Default|GetTurnsToCapture))
          (return)))
      (:Completed
        (if (Utilities|Enum|Equal(Enum) (LocalVariables|GetfirstUnit) (Variables|Default|GetPrevousTeam))
          (Math|Integer|DecrementInt (Variables|Default|GetTurnsLeft)
            (:%20%20
              _))
          (else
            (bind _output_get (Variables|Default|SetTurnsLeft (Variables|Default|GetTurnsToCapture)))
            (Math|Integer|DecrementInt _output_get
              (:%20%20
                _))))
        (Variables|Default|SetPrevousTeam (LocalVariables|GetfirstUnit))))))