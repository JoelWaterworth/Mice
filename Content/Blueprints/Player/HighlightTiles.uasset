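; HighlightTiles displays highlights over a set of grid tiles using instances in HighlightPool.
; UpdateTilesFor clears the pool, then adds an instance slightly above the centre of each tile in the passed map's keys, on a 100-unit grid; Deselect clears it.
; Construction pre-fills the pool with hidden far-off instances.
; MoveOffScreen, not called in this file, relocates instances off-screen, dirtying render state only on the last update.
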(event Custom|UpdateTilesFor
  (params (NewParam :type Map%20of%20Int%20Vector%20Structures%20to%20Structs))
  (Components|InstancedStaticMesh|ClearInstances (Variables|Default|GethighlightPool))
  (bind _keys (Utilities|Map|Keys NewParam))
  (bind _output (Utilities|ForEachLoopwithLast _keys)
    (:then_0
      _)
    (:Last
      _))
  (Class|InstancedStaticMeshComponent|AddInstanceWorldSpace (Variables|Default|GethighlightPool) (Math|Transform|MakeTransform (+ (* (Math|Conversions|ToVector(Float) _output) 1e+02) "50.000000,50.000000,10.000000") "0, 0, 0" "1,1,1")))

(event Custom|Deselect
  (Components|InstancedStaticMesh|ClearInstances (Variables|Default|GethighlightPool)))

(fn ConstructionScript
  (for _index (range 0 100)
    (Components|InstancedStaticMesh|AddInstance (Variables|Default|GethighlightPool) (Math|Transform|MakeTransform "-1000.000000,-1000.000000,-1000.000000" "0, 0, 0" "1,1,1"))))

(fn MoveOffScreen
  (bind _offscreem (Variables|Default|GetOffScreem))
  (bind _variable (Utilities|ForLoopwithLast 0 (Components|InstancedStaticMesh|GetInstanceCount (Variables|Default|GethighlightPool)))
    (:Body
      (Components|InstancedStaticMesh|UpdateInstanceTransform (Variables|Default|GethighlightPool) _variable (Math|Transform|MakeTransform _offscreem "0, 0, 0" "1,1,1") true false true))
    (:Last
      (Components|InstancedStaticMesh|UpdateInstanceTransform (Variables|Default|GethighlightPool) _variable (Math|Transform|MakeTransform _offscreem "0, 0, 0" "1,1,1") false true true))))