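; Path actor that draws its owning BPUnit's route as a mesh ribbon and destroys itself when the unit finishes the path.
; On BeginPlay it binds to the unit's finish event and calls Update with its Path array.
; Update scales grid coordinates into raised spline points, then lays spline mesh segments at fixed distance intervals along the spline.
; Spawned segments are tracked in Waste so each rebuild can clear them first.
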(event Custom|Path%20Finished
  (Actor|DestroyActor))

(event EventBeginPlay
  (bind _asbpunit (Utilities|Casting|CastToBPUnit (Components|GetOwner))
    (:then
      (EventDispatchers|BindEventtoFinishPath _asbpunit (delegate Custom|Path%20Finished))
      (CallFunction|Update (Variables|Default|GetPath)))
    (:CastFailed
      (Development|PrintString "Cast failed"))))

(fn ConstructionScript)

(fn Update
  (params (TargetArray :type Array%20of%20Int%20Vector%20Structures))
  (bind _spline (Variables|Default|GetSpline))
  (bind _waste (Variables|Default|GetWaste))
  (bind _spline_2 (Variables|Default|GetSpline))
  (Utilities|FlowControl|Sequence
    (:then_0
      (for _array_element _waste
        (Components|DestroyComponent _array_element))
      (Utilities|Array|Clear _waste)
      (Spline|ClearSplinePoints (Variables|Default|GetSpline) true)
      (for (_array_element_2 _array_index) TargetArray
        (Class|SplineComponent|AddPoint (Variables|Default|GetSpline) (Utilities|Struct|MakeSplinePoint (Math|Conversions|ToFloat(Integer) _array_index) (+ (* (Math|Conversions|ToVector(Float) _array_element_2) 1e+02) (Math|Vector|MakeVector 0.0 0.0 (Variables|Default|Getpath%20height)))) false))
      (Spline|UpdateSpline (Variables|Default|GetSpline)))
    (:then_1
      (for _index (range 0 (Math|Float|Floor (/ (Spline|GetSplineLength (Variables|Default|GetSpline)) 1e+02)))
        (bind _returnvalue (AddComponent|AddSplineMeshComponent true (Transformation|GetActorTransform)))
        (Components|StaticMesh|SetStaticMesh _returnvalue (Variables|Default|Getmesh))
        (Rendering|Material|SetMaterial _returnvalue 0 (Variables|Default|GetMaterial%20Instance))
        (SplineMesh|SetStartandEnd _returnvalue (Spline|GetLocationatDistanceAlongSpline _spline (Math|Conversions|ToFloat(Integer) (* _index 100)) "Local") (Spline|GetTangentatDistanceAlongSpline _spline (Math|Conversions|ToFloat(Integer) (* _index 100)) "Local") (Spline|GetLocationatDistanceAlongSpline _spline_2 (+ (Math|Conversions|ToFloat(Integer) (* _index 100)) 1e+02) "Local") (Spline|GetTangentatDistanceAlongSpline _spline_2 (+ (Math|Conversions|ToFloat(Integer) (* _index 100)) 1e+02) "Local") true :!class /Script/Engine.SplineMeshComponent)
        (Utilities|Array|Add (Variables|Default|GetWaste) _returnvalue)))))