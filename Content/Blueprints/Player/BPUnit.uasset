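; Team-colored unit for a grid-based tactics game, with tile movement, cover, shooting and overwatch.
; Tick walks it along a tile path, firing OnNewTile, which enemy units bind on the authority to trigger overwatch shots.
; Shot probability uses a voxel line trace against walls and obstacles plus a weapon distance curve; units in cover can test shots from adjacent tiles.
; Helpers spawn phantom and path previews; lethal damage destroys the unit.
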(event Custom|Finished
  (Variables|Default|SetcurrentState "US_Idle")
  (Networking|SwitchHasAuthority
    (:Remote
      (Default|CallFinishPath))))

(event Custom|EnemyOnNewTile
  (params (NewParam :type BP%20Unit%20Object%20Reference))
  (Development|PrintString "EnemyOnNewTile")
  (if (Variables|Default|GetInOverwatch)
    (CallFunction|OnOverwatch NewParam)))

(event Custom|OnOverwatch
  (params (NewParam :type BP%20Unit%20Object%20Reference))
  (bind _returnvalue (Transformation|GetActorLocation NewParam))
  (bind _returnvalue_2 (Transformation|GetActorLocation))
  (bind _newparam (CallFunction|CalculateProbabiltyOfShoot _returnvalue_2 _returnvalue))
  (if (> _newparam 5.0)
    (CallFunction|FireShot _newparam NewParam)))

(event EventBeginPlay
  (Utilities|FlowControl|Delay 0.5)
  (Utilities|FlowControl|Sequence
    (:then_0
      (Rendering|Material|SetMaterial (Variables|Character|GetMesh) 0 (Utilities|Select :Index (Variables|Default|Getteam) :T_Blue "/Game/Materials/Blue.Blue" :T_Red "/Game/Materials/Red.Red"))
      (CallFunction|SetIsinCover))
    (:then_1
      (Networking|SwitchHasAuthority
        (:Authority
          (bind _outactors (Actor|GetAllActorsOfClass "BPUnit_C"))
          (for _array_element _outactors
            (if (not (Utilities|Enum|Equal(Enum) (Variables|/Script/Mice.Unit|Getteam _array_element) (Variables|Default|Getteam)))
              (EventDispatchers|BindEventtoOnNewTile _array_element (delegate Custom|EnemyOnNewTile))
              (Development|PrintString "BindOnNewTile"))))))))

(event Game|Damage|EventAnyDamage
  (params (Damage :type Float%20%28single-precision%29) (DamageType :type Damage%20Type%20Object%20Reference) (InstigatedBy :type Controller%20Object%20Reference) (DamageCauser :type Actor%20Object%20Reference))
  (bind _output_get (Variables|Default|SetHealth (- (Variables|Default|GetHealth) (Math|Float|Truncate Damage))))
  (if (<= _output_get 0)
    (Actor|DestroyActor)))

(event EventTick
  (params (DeltaSeconds :type Float%20%28single-precision%29))
  (bind _returnvalue (Transformation|GetActorLocation))
  (bind _self self)
  (bind _next_location (Variables|Default|GetNext%20location))
  (bind _x (Variables|Default|Getx))
  (bind _paths (Variables|Default|GetPaths))
  (bind _returnvalue_2 (- _next_location _returnvalue))
  (bind (_x_2 _y) (Math|Vector|BreakVector _returnvalue_2))
  (bind _returnvalue_3 (Math|Vector|MakeVector _x_2 _y 0.0))
  (bind _returnvalue_4 (Math|Conversions|ToVector2D(Vector) _returnvalue_3))
  (bind _returnvalue_5 (Math|Vector2D|Vector2DLength _returnvalue_4))
  (switch Utilities|FlowControl|Switch|SwitchonEUnitState (Variables|Default|GetcurrentState)
    (:US_Walk
      (Transformation|SetActorRotation (Math|Rotator|CombineRotators "0,-90.000000, 0" (Math|Conversions|RotationFromXVector _returnvalue_3)))
      (if (<= _returnvalue_5 2.0)
        (Variables|Default|Setpos (Utilities|Array|Get(acopy) _paths _x) :!label _label)
        (bind _result (Math|Integer|IncrementInt _x)
          (:%20%20
            (Default|CallOnNewTile _self _self)
            (if (>= _result (Utilities|Array|Length _paths))
              (CallFunction|Finished)
              (else
                (CallFunction|SetNewLocation)))))
        (elif (and (<= _returnvalue_5 5.0) (< (+ (Variables|Default|Getx) 1) (Utilities|Array|Length (Variables|Default|GetPaths))))
          (goto _label)
          (else
            (Pawn|Input|AddMovementInput (Math|Vector|Normalize _returnvalue_3) (select (< _returnvalue_5 1e+01) (Math|Float|Lerp 1.0 0.0 _returnvalue_5) 1.0) true)))))))

(fn ConstructionScript)

(fn Goto
  (params (Paths :type Array%20of%20Int%20Vector%20Structures))
  (Variables|Default|Setx 0)
  (Variables|Default|SetcurrentState "US_Walk")
  (Variables|Default|SetPaths Paths)
  (CallFunction|SetNewLocation))

(fn SetNewLocation
  (Variables|Default|SetNext%20location (+ (* (Math|Conversions|ToVector(Float) (Utilities|Array|Get(acopy) (Variables|Default|GetPaths) (Variables|Default|Getx))) 1e+02) (Math|Vector|MakeVector 5e+01 5e+01 (Components|Capsule|GetScaledCapsuleHalfHeight (Variables|Default|GetCapsuleComponent))))))

(fn CalculateProbabiltyOfShoot
  (params (start :type Vector) (end :type Vector))
  (LocalVariables|Seta_start (/ start 1e+02))
  (bind _output_get (LocalVariables|SetaEnd (/ end 1e+02)))
  (LocalVariables|SetendTile (Utilities|VectortoIntVector _output_get))
  (bind _outactors (Actor|GetAllActorsOfClass "/Script/Mice.WorldGrid"))
  (LocalVariables|SetworldGrid (Utilities|Array|Get(acopy) _outactors))
  (bind _returnvalue (Game|ConstructObjectfromClass "/Script/Mice.VoxelLineTraceIterator" self))
  (bind _output_get_2 (LocalVariables|SetIterator _returnvalue))
  (Variables|/Script/Mice.VoxelLineTraceIterator|Setstart _output_get_2 (LocalVariables|Geta_start))
  (Variables|/Script/Mice.VoxelLineTraceIterator|Setdirection _output_get_2 (- (LocalVariables|GetaEnd) (LocalVariables|Geta_start)))
  (while (LocalVariables|GetContinue)
    (bind _returnvalue_2 (Class|VoxelLineTraceIterator|Next (LocalVariables|GetIterator)))
    (for _array_element (.in_voxels _returnvalue_2)
      (for _array_element_2 (.direction _array_element)
        (if (Utilities|Map|Contains (Class|WorldGrid|GetWallObstucles (LocalVariables|GetworldGrid)) (Utilities|Struct|MakeBoarderKey _array_element_2 (.voxel _array_element)))
          (return 0.0)
          (else
            (Development|PrintString (Utilities|String|Append (Utilities|String|EnumtoString _array_element_2) "     " (Utilities|String|ToString(Integer) (.voxel _array_element))) true true "(R=0.000000,G=0.660000,B=1.000000,A=1.000000)" 1e+01))))
      (if (Utilities|Eq (.voxel _array_element) (LocalVariables|GetendTile))
        (return (Math|Curves|GetFloatValue (.curve (Utilities|Struct|BreakWeaponInfo (Variables|Default|GetWeaponInfo))) (Math|Vector|VectorLength (/ (- end start) 1e+02))))
        (elif (Utilities|Map|Contains (Class|WorldGrid|GetObstucles (LocalVariables|GetworldGrid)) (.voxel _array_element))
          (return 0.0))))))

(fn Applystack
  (params (NewParam2 :type Float%20%28single-precision%29) (NewParam :type Array%20of%20Probabilty%20Effect%20Object%20References))
  (LocalVariables|SetNewLocalVar_1 NewParam2)
  (bind _arrayelement (Utilities|Array|ReverseforEachLoop NewParam)
    (:LoopBody
      (bind _newparam1 (Default|Apply _arrayelement (LocalVariables|GetNewLocalVar_1)))
      (LocalVariables|SetNewLocalVar_1 _newparam1))
    (:Completed
      (return (LocalVariables|GetNewLocalVar_1)))))

(fn FindBestAngleOfShoot
  (params (Target :type BP%20Unit%20Object%20Reference))
  (LocalVariables|SetEnd (+ "0, 0, 0" (Transformation|GetActorLocation Target)))
  (bind _output_get (LocalVariables|Setstartx (+ "0, 0, 0" (Transformation|GetActorLocation self))))
  (if (and (not (Variables|Default|GetisInCover)) (> (CallFunction|CalculateProbabiltyOfShoot _output_get (LocalVariables|GetEnd)) 0.0))
    (return (CallFunction|CalculateProbabiltyOfShoot _output_get (LocalVariables|GetEnd)) (LocalVariables|Getstartx))
    (else
      (bind _index (Utilities|FlowControl|ForLoopwithBreak -1 1)
        (:LoopBody
          (for _index_2 (range -1 1)
            (if (not (and (== _index_2 0) (== _index 0)))
              (bind _outactors (Actor|GetAllActorsOfClass "/Game/Blueprints/BPWorldGrid.BPWorldGrid_C"))
              (if (Utilities|Map|Contains (Variables|/Script/Mice.WorldGrid|GetgridTiles (Utilities|Array|Get(acopy) _outactors)) (Utilities|VectortoIntVector (/ (+ (* (Math|Vector|MakeVector (Math|Conversions|ToFloat(Integer) _index_2) (Math|Conversions|ToFloat(Integer) _index) 0.0) 1e+02) (Transformation|GetActorLocation self)) 1e+02)))
                (if (> (CallFunction|CalculateProbabiltyOfShoot (LocalVariables|Getstartx) (+ (LocalVariables|Getstartx) (* (Math|Vector|MakeVector (Math|Conversions|ToFloat(Integer) _index_2) (Math|Conversions|ToFloat(Integer) _index) 0.0) 1e+02))) 0.0)
                  (if (> (CallFunction|CalculateProbabiltyOfShoot (+ (LocalVariables|Getstartx) (* (Math|Vector|MakeVector (Math|Conversions|ToFloat(Integer) _index_2) (Math|Conversions|ToFloat(Integer) _index) 0.0) 1e+02)) (LocalVariables|GetEnd)) 0.0)
                    (return (CallFunction|CalculateProbabiltyOfShoot (+ (LocalVariables|Getstartx) (* (Math|Vector|MakeVector (Math|Conversions|ToFloat(Integer) _index_2) (Math|Conversions|ToFloat(Integer) _index) 0.0) 1e+02)) (LocalVariables|GetEnd)) (+ (LocalVariables|Getstartx) (* (Math|Vector|MakeVector (Math|Conversions|ToFloat(Integer) _index_2) (Math|Conversions|ToFloat(Integer) _index) 0.0) 1e+02)))))))))
        (:Completed
          (return 0.0 (LocalVariables|Getstartx)))))))

(fn SetIsinCover
  (bind (_x _y) (Utilities|Neghbours)
    (:Loop%20Body
      (bind _outactors (Actor|GetAllActorsOfClass "/Game/Blueprints/BPWorldGrid.BPWorldGrid_C"))
      (if (Utilities|Map|Contains (Class|WorldGrid|GetObstucles (Utilities|Array|Get(acopy) _outactors)) (Utilities|VectortoIntVector (/ (+ (* (Math|Vector|MakeVector (Math|Conversions|ToFloat(Integer) _x) (Math|Conversions|ToFloat(Integer) _y) 1.0) 1e+02) (Transformation|GetActorLocation)) 1e+02)))
        (Variables|Default|SetisInCover true)
        (return)))
    (:Complete
      (Variables|Default|SetisInCover false))))

(fn SpawnPhantom
  (params (SpawnTransform :type Transform))
  (Game|SpawnActorfromClass "/Game/Blueprints/Player/Phantom.Phantom_C" SpawnTransform "AlwaysSpawn" self 0))

(fn GetCurrentTile
  (return (Variables|Default|GetCurrentTile)))

(fn CreatePath
  (params (InputPin :type Vector) (Target :type BP%20Unit%20Object%20Reference))
  (bind _returnvalue (Game|SpawnActorfromClass "/Script/CableComponent.CableActor" (Math|Transform|MakeTransform "0, 0, 0" "0, 0, 0" "1,1,1") "AlwaysSpawn" 0 0))
  (Variables|/Script/CableComponent.CableComponent|SetCableGravityScale (Variables|/Script/CableComponent.CableActor|GetCableComponent _returnvalue) 0.0)
  (Variables|/Script/CableComponent.CableComponent|SetSolverIterations (Variables|/Script/CableComponent.CableActor|GetCableComponent _returnvalue) 10)
  (Variables|/Script/CableComponent.CableComponent|SetEndLocation (Variables|/Script/CableComponent.CableActor|GetCableComponent _returnvalue) (- (+ "0, 0, 0" (Transformation|GetActorLocation Target)) InputPin))
  (return _returnvalue))

(fn FireShot
  (params (probability :type Float%20%28single-precision%29) (target :type BP%20Unit%20Object%20Reference))
  (if (> (Math|Random|RandomFloatinRange 0.0 1e+02) probability)
    (Game|Damage|ApplyDamage target (Math|Conversions|ToFloat(Integer) (.Damage (Utilities|Struct|BreakWeaponInfo (Variables|Default|GetWeaponInfo)))) 0 0)
    (Development|PrintString "Hit")
    (else
      (Development|PrintString "Miss"))))

(fn SpawnPath
  (params (start :type Int%20Vector%20Structure) (Path :type Array%20of%20Int%20Vector%20Structures) (end :type Vector) (NewParam :type Phantom%20Object%20Reference%20%28by%20ref%29))
  (bind _self self)
  (bind _output_get (LocalVariables|SetNewLocalVar_2 Path))
  (Utilities|Array|Insert _output_get start)
  (if (and (Utilities|IsValid NewParam) (Utilities|IsValid (Variables|Default|GetPath)))
    (Default|Update (Variables|Default|GetPath) (LocalVariables|GetNewLocalVar_2))
    (else
      (bind _returnvalue (Game|SpawnActorfromClass "/Game/Blueprints/Player/Phantom.Phantom_C" (Math|Transform|MakeTransform end "0, 0, 0" "1,1,1") "AlwaysSpawn" _self 0))
      (|SetBy-RefVar NewParam _returnvalue)
      (bind _returnvalue_2 (Game|SpawnActorfromClass "/Game/Blueprints/Player/Path.Path_C" (Math|Transform|MakeTransform "50.000000,50.000000, 0" "0, 0, 0" "1,1,1") "AlwaysSpawn" _self (LocalVariables|GetNewLocalVar_2) 0))
      (Variables|Default|SetPath _returnvalue_2))))