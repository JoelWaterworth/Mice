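; Player controller for a multiplayer, turn-based grid tactics game, handling unit selection, command input, HUD and game-over screen.
; Selecting a team unit caches reachable routes from the world grid and broadcasts them for tile highlighting.
; Tick snaps cursor hits to grid tiles by searching down in Z, previewing moves with a phantom and path actor.
; Walk, shoot and overwatch orders become command objects on authority, submitted to the turn game state.
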(event Custom|CreateWalkCommand
  (params (NewParam2 :type BP%20Unit%20Object%20Reference) (path :type Array%20of%20Int%20Vector%20Structures))
  ;[1 1 1] Create Walk Command
  (Networking|SwitchHasAuthority
    (:Authority
      (bind _returnvalue (Game|ConstructObjectfromClass "/Game/Blueprints/Player/WalkCommand.WalkCommand_C" self))
      (Variables|/Game/Blueprints/Player/WalkCommand.WalkCommand_C|Setunit _returnvalue NewParam2)
      (Variables|/Game/Blueprints/Player/WalkCommand.WalkCommand_C|Setpath _returnvalue path)
      (CallFunction|AddCommand _returnvalue NewParam2))))

(event Custom|CreateShootCommand
  (params (T :type BP%20Unit%20Object%20Reference) (Prob :type Float%20%28single-precision%29) (Shooter :type BP%20Unit%20Object%20Reference))
  ;[1 1 1] Create Shoot Command
  (Networking|SwitchHasAuthority
    (:Authority
      (bind _returnvalue (Game|ConstructObjectfromClass "/Game/Blueprints/Player/ShootCommand.ShootCommand_C" self T Shooter Prob))
      (Utilities|IsValid T
        (:Is%20Valid
          (CallFunction|AddCommand _returnvalue T))
        (:Is%20Not%20Valid
          (Development|PrintString "Target invalid"))))))

(event Custom|OnSelect_Event
  (params (tiles :type Map%20of%20Int%20Vector%20Structures%20to%20Structs))
  ;[1 1 1] Event Begin
  (bind _output (Utilities|GetHighlight)
    (:Is%20Valid
      (Default|UpdateTilesfor _output tiles))
    (:Is%20Not%20Valid
      (Development|PrintString "No Highlights"))))

(event Custom|GameOver_Event_0
  (params (team%20that%20won :type ETeam%20Enum :default "T_Blue"))
  ;[1 1 1] Event Begin
  (Widget|RemovefromParent (Variables|Default|GetGUI))
  (bind _returnvalue (UserInterface|CreateWidget "/Game/Blueprints/HUD/GameOver.GameOver_C" self team%20that%20won))
  (UserInterface|Viewport|AddtoViewport _returnvalue 1))

(event Custom|AddOverwatch
  (params (S :type BP%20Unit%20Object%20Reference))
  ;[1 1 1] Overwacth
  (Networking|SwitchHasAuthority
    (:Authority
      (bind _returnvalue (Game|ConstructObjectfromClass "/Game/Blueprints/Player/OverwatchCommand.OverwatchCommand_C" self S))
      (CallFunction|AddCommand _returnvalue S))))

(event Custom|TurnOver
  (params (NewParam :type ETeam%20Enum :default "T_Blue"))
  (bind _asmplayer_state (Utilities|Casting|CastToMPlayerState (Variables|Default|GetPlayerState)))
  (Default|NowWaitingon (Variables|Default|GetGUI) (== (Variables|/Script/Mice.MPlayerState|Getteam _asmplayer_state) NewParam))
  (if (== (Variables|/Script/Mice.MPlayerState|Getteam _asmplayer_state) NewParam)
    (bind _unit (CallFunction|GetNextUnit))
    (CallFunction|SelectUnit _unit)
    (else
      (bind _output (Utilities|GetHighlight)
        (:Is%20Valid
          (Default|Deselect _output)
          (Development|PrintString "Deselect"))))))

(event EventBeginPlay
  (bind _returnvalue (Networking|IsDedicatedServer))
  ;[1 1 1] Event Begin
  (Networking|SwitchHasAuthority
    (:Authority
      (Development|PrintString (select _returnvalue "Dedicated Server" "Listen Server") true true "(R=0.000000,G=0.660000,B=1.000000,A=1.000000)" 2e+01)
      (if (not _returnvalue)
        (if (Pawn|IsLocalPlayerController)
          (Utilities|FlowControl|Sequence :!label _label
            (:then_0
              (bind _output (Utilities|GetWorldGrid)
                (:Us%20Valid
                  (bind _returnvalue_2 (Game|SpawnActorfromClass "/Game/Blueprints/Player/cursor.cursor_C" (Class|WorldGrid|VectortoWorldTransform _output) "AlwaysSpawn" 0 0))
                  (Variables|Default|Setcursor _returnvalue_2)
                  (bind _returnvalue_3 (UserInterface|CreateWidget "/Game/Blueprints/HUD/BPWidget.BPWidget_C" self))
                  (bind _output_get (Variables|Default|SetGUI _returnvalue_3))
                  (UserInterface|Viewport|AddtoViewport _output_get 0))))
            (:then_1
              (EventDispatchers|BindEventtoOnSelect (delegate Custom|OnSelect_Event)))
            (:then_2
              (Utilities|FlowControl|Delay 1.0)
              (bind _asmplayer_state (Utilities|Casting|CastToMPlayerState (Variables|Default|GetPlayerState)))
              (bind _unit (Utilities|GetUnitsOfTeam (Variables|/Script/Mice.MPlayerState|Getteam _asmplayer_state))
                (:Body
                  (CallFunction|SelectUnit _unit))))
            (:then_3
              (bind _asbpturn_game_state (Utilities|Casting|CastToBPTurnGameState (Game|GetGameState)))
              (EventDispatchers|AssignGameOver _asbpturn_game_state (delegate Custom|GameOver_Event_0)))))))
    (:Remote
      (goto _label))))

(event EventTick
  (params (DeltaSeconds :type Float%20%28single-precision%29))
  (bind (_hitresult _returnvalue) (Game|Player|GetHitResultUnderCursorbyChannel "TraceTypeQuery1" true))
  (bind _selected (Variables|Default|Getselected))
  ;[1 1 1] Tick
  (Networking|SwitchHasAuthority
    (:Authority
      (if (Pawn|IsLocalPlayerController)
        (if _returnvalue :!label _label
          (bind _outputpin (Utilities|NewMacro0 5 _hitresult :!label _label_2)
            (:true
              (if (not (CallFunction|Eq (Variables|Default|GetHoverPos) _outputpin))
                (bind _output_get (Variables|Default|SetHoverPos _outputpin))
                (Utilities|IsValid (Variables|Default|Getcursor)
                  (:Is%20Valid
                    (Utilities|IsValid _selected
                      (:Is%20Valid
                        (if (Math|Boolean|ANDBoolean (not (Variables|/Script/Mice.Unit|GetbHasExecutedCommand _selected)) (not (Variables|Default|GetbInCommandBar)) (> (Utilities|Array|Length (Class|WorldGrid|CreatePathfromRoutes (Variables|Default|GetPaths) _output_get)) 0))
                          (CallFunction|UpdatePhantom _selected (* (+ (Math|Conversions|ToVector(Float) _output_get) "0.500000,0.500000, 0") 1e+02) (Class|WorldGrid|CreatePathfromRoutes (Variables|Default|GetPaths) _output_get) (Variables|/Script/Mice.Unit|Getpos _selected))
                          (goto _label_2 Break))))))))))))
    (:Remote
      (goto _label))))

(event EventUpdatePlayerTeam
  (params (team :type ETeam%20Enum :default "T_Blue"))
  (bind _gui (Variables|Default|GetGUI))
  ;[1 1 1] UpdatePlayerTeam
  (Utilities|IsValid _gui
    (:Is%20Valid
      (Default|UpdateColours _gui team))))

(event Input|ActionEvents|InputActionSelect
  (params (Key :type Key%20Structure))
  (bind (_hitresult _returnvalue) (Game|Player|GetHitResultUnderCursorbyChannel "TraceTypeQuery1" true))
  ;[1 1 1] Select
  (:Pressed
    (if _returnvalue
      (bind _asbpunit (Utilities|Casting|CastToBPUnit (.HitActor (Collision|BreakHitResult _hitresult))))
      (bind _asmplayer_state (Utilities|Casting|CastToMPlayerState (Variables|Default|GetPlayerState)))
      (if (Utilities|Enum|Equal(Enum) (Variables|/Script/Mice.MPlayerState|Getteam _asmplayer_state) (Variables|/Script/Mice.Unit|Getteam _asbpunit))
        (CallFunction|SelectUnit _asbpunit)))))

(event Input|ActionEvents|InputActionTarget
  (params (Key :type Key%20Structure))
  (bind (_hitresult _returnvalue) (Game|Player|GetHitResultUnderCursorbyChannel "TraceTypeQuery1" true))
  ;[1 1 1] Target
  (:Pressed
    (if _returnvalue
      (bind _outputpin (Utilities|NewMacro0 5 _hitresult :!label _label)
        (:true
          (if (> (Utilities|Array|Length (Class|WorldGrid|CreatePathfromRoutes (Variables|Default|GetPaths) _outputpin)) 0)
            (CallFunction|CreateWalkCommand (Variables|Default|Getselected) (Class|WorldGrid|CreatePathfromRoutes (Variables|Default|GetPaths) _outputpin))
            (bind (_available_unit _unit) (CallFunction|GetNextUnit))
            (if _available_unit
              (CallFunction|SelectUnit _unit)
              (goto _label Break))))))))

(event Input|ActionEvents|InputActionEsc
  (params (Key :type Key%20Structure))
  (:Pressed
    (Default|Escape (Variables|Default|GetGUI))))

(fn ConstructionScript)

(fn AddCommand
  (params (command :type M%20Command%20Object%20Reference) (target :type Unit%20Object%20Reference))
  (Variables|/Script/Mice.Unit|Setcommand target command)
  (bind _asbpturn_game_state (Utilities|Casting|CastToBPTurnGameState (Game|GetGameState)))
  (Class|MGameState|SumbitCommand _asbpturn_game_state self target))

(fn GetNextUnit
  (bind _asmplayer_state (Utilities|Casting|CastToMPlayerState (Variables|Default|GetPlayerState)))
  (bind _unit (Utilities|GetUnitsOfTeam (Variables|/Script/Mice.MPlayerState|Getteam _asmplayer_state))
    (:Body
      (if (Variables|/Script/Mice.Unit|GetbHasExecutedCommand _unit)
        (return true _unit)))
    (:Complete
      (return false 0))))

(fn SelectUnit
  (params (InputPin :type BP%20Unit%20Object%20Reference))
  (Utilities|IsValid InputPin
    (:Is%20Valid
      (Utilities|IsValid (Variables|Default|Getselected)
        (:Is%20Valid
          (Rendering|SetVisibility (Variables|/Script/Mice.Unit|GetselectPlane (Variables|Default|Getselected)) false false))
        (:Is%20Not%20Valid
          _))
      (bind _output (Utilities|GetWorldGrid)
        (:Us%20Valid
          (bind _returnvalue (Class|WorldGrid|CalculatePaths _output InputPin 8))
          (bind _output_get (Variables|Default|SetPaths _returnvalue))
          (bind _output_get_2 (Variables|Default|Setselected InputPin))
          (Default|CallOnSelect _output_get)
          (Rendering|SetVisibility (Variables|/Script/Mice.Unit|GetselectPlane _output_get_2) true false))))))

(fn UpdatePhantom
  (params (unit :type BP%20Unit%20Object%20Reference) (End :type Vector) (Path :type Array%20of%20Int%20Vector%20Structures) (start :type Int%20Vector%20Structure))
  (bind _self self)
  (bind _output_get (LocalVariables|SetLocPath Path))
  (Utilities|Array|Insert _output_get start)
  (if (and (Utilities|IsValid (Variables|Default|GetPhantom)) (Utilities|IsValid (Variables|Default|GetPath)))
    (Default|Update (Variables|Default|GetPath) (LocalVariables|GetLocPath))
    (Transformation|SetActorTransform (Variables|Default|GetPhantom) (Math|Transform|MakeTransform End "0, 0, 0" "1,1,1") false true)
    (else
      (bind _returnvalue (Game|SpawnActorfromClass "/Game/Blueprints/Player/Phantom.Phantom_C" (Math|Transform|MakeTransform End "0, 0, 0" "1,1,1") "AlwaysSpawn" _self 0))
      (Variables|Default|SetPhantom _returnvalue)
      (bind _returnvalue_2 (Game|SpawnActorfromClass "/Game/Blueprints/Player/Path.Path_C" (Math|Transform|MakeTransform "50.000000,50.000000, 0" "0, 0, 0" "1,1,1") "AlwaysSpawn" _self (LocalVariables|GetLocPath) 0))
      (Variables|Default|SetPath _returnvalue_2))))