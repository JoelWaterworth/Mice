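; BPRoof is a roof actor that hides itself in game while units are inside the box volume beneath it.
; A construction script sizes the box from BoxVector and offsets it downward, and a unit entering it triggers hiding.
; BeginPlay, visible units leaving and destruction of overlapping units re-scan the box, which sets roof visibility based on non-hidden units.
; OnDestroyed bindings on overlapping units cover units that die inside.
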(event OnComponentBeginOverlap(Box)
  (params (OverlappedComponent :type Primitive%20Component%20Object%20Reference) (OtherActor :type Actor%20Object%20Reference) (OtherComp :type Primitive%20Component%20Object%20Reference) (OtherBodyIndex :type Integer) (bFromSweep :type Boolean) (SweepResult :type Hit%20Result%20Structure%20%28by%20ref%29))
  (bind _asbpunit (Utilities|Casting|CastToBPUnit OtherActor))
  (Game|BindEventtoOnDestroyed _asbpunit (delegate Custom|Overlapping%20Actor%20Destroyed))
  (if (not (Variables|/Script/Engine.Actor|GetbHidden _asbpunit))
    (Rendering|SetActorHiddenInGame true)
    (elif (not (Variables|Rendering|GetbHidden))
      (Rendering|SetActorHiddenInGame true))))

(event OnComponentEndOverlap(Box)
  (params (OverlappedComponent :type Primitive%20Component%20Object%20Reference) (OtherActor :type Actor%20Object%20Reference) (OtherComp :type Primitive%20Component%20Object%20Reference) (OtherBodyIndex :type Integer))
  (bind _asbpunit (Utilities|Casting|CastToBPUnit OtherActor))
  (if (not (Variables|/Script/Engine.Actor|GetbHidden _asbpunit))
    (CallFunction|UpdateOvelappingActors (delegate Custom|Overlapping%20Actor%20Destroyed))
    (Game|UnbindEventfromOnDestroyed OtherActor (delegate Custom|Overlapping%20Actor%20Destroyed))))

(event Custom|Overlapping%20Actor%20Destroyed
  (params (DestroyedActor :type Actor%20Object%20Reference))
  (CallFunction|UpdateOvelappingActors (delegate Custom|Overlapping%20Actor%20Destroyed))
  (Game|UnbindEventfromOnDestroyed (stale OnComponentEndOverlap(Box) OtherActor) (delegate Custom|Overlapping%20Actor%20Destroyed)))

(event EventBeginPlay
  (CallFunction|UpdateOvelappingActors (delegate Custom|Overlapping%20Actor%20Destroyed)))

(fn ConstructionScript
  (bind _box (Variables|Default|GetBox))
  (bind _boxvector (Variables|Default|GetBoxVector))
  (Components|Box|SetBoxExtent _box _boxvector true)
  (Transformation|SetRelativeLocation _box (Math|Vector|MakeVector 0.0 0.0 (* (.Z (Math|Vector|BreakVector _boxvector)) -1.0)) false false))

(fn UpdateOvelappingActors
  (params (Delegate :type Delegate%20%28by%20ref%29))
  (for _array_element (Collision|GetOverlappingActors (Variables|Default|GetBox) "/Script/Mice.Unit" :!class /Script/Engine.PrimitiveComponent)
    (Game|BindEventtoOnDestroyed _array_element Delegate)
    (if (not (Variables|/Script/Engine.Actor|GetbHidden _array_element))
      (LocalVariables|SetHidden true)))
  (Rendering|SetActorHiddenInGame (LocalVariables|GetHidden)))