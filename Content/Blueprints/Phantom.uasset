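; Phantom actor that displays a static-mesh copy of its owner until that owner comes close.
; On BeginPlay it duplicates the owner's static mesh components tagged "Phantom" at their relative transforms, applying an override material to each copy's first slot.
; Each tick it measures the distance to the owner and destroys itself once that is within MinDistance.
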(event EventBeginPlay
  (for _array_element (Actor|GetComponentsbyTag (Components|GetOwner) "/Script/Engine.StaticMeshComponent" "Phantom")
    (bind _returnvalue (AddComponent|AddStaticMeshComponent false (Transformation|GetRelativeTransform _array_element)))
    (Components|StaticMesh|SetStaticMesh _returnvalue (Variables|/Script/Engine.StaticMeshComponent|GetStaticMesh _array_element))
    (Rendering|Material|SetMaterial _returnvalue 0 (Variables|Default|GetNewVar_0))))

(event EventTick
  (params (DeltaSeconds :type Float%20%28single-precision%29))
  (if (>= (Variables|Default|GetMinDistance) (Math|Vector|VectorLength (- (Transformation|GetActorLocation (Components|GetOwner)) (Transformation|GetActorLocation))))
    (Actor|DestroyActor)))

(fn ConstructionScript)