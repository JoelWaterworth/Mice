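; BPUnit is a unit actor that walks tile by tile along a grid path handed to it.
; MoveTo drops the path's last entry, then walks the remaining entries from the end back to index zero, returning to Idle when done.
; Tick moves it at constant Speed without sweep, snapping to each waypoint and recording its grid position.
; Waypoint world locations come from the first BPWorldGrid found in the level.
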(event EventBeginPlay)

(event Collision|EventActorBeginOverlap
  (params (OtherActor :type Actor%20Object%20Reference)))

(event EventTick
  (params (DeltaSeconds :type Float%20%28single-precision%29))
  (bind _returnvalue (Transformation|GetActorLocation))
  (bind _next_location (Variables|Default|GetNext%20location))
  (bind _speed (Variables|Default|Getspeed))
  (bind _returnvalue_2 (- _next_location _returnvalue))
  (bind _returnvalue_3 (* DeltaSeconds _speed))
  (bind _returnvalue_4 (Math|Vector|Normalize _returnvalue_2))
  (bind _returnvalue_5 (* _returnvalue_4 _returnvalue_3))
  (switch Utilities|FlowControl|Switch|SwitchonUnitState (Variables|Default|Getstate)
    (:NewEnumerator1
      (if (< (Math|Vector|VectorLength _returnvalue_2) (Math|Vector|VectorLength _returnvalue_5))
        (Transformation|SetActorLocation (Variables|Default|GetNext%20location) false false)
        (Variables|Default|Setpos (Utilities|Array|Get(acopy) (Variables|Default|GetPath) (Variables|Default|GetPathPos)))
        (bind _output_get (Variables|Default|SetPathPos (- (Variables|Default|GetPathPos) 1)))
        (if (< _output_get 0)
          (Variables|Default|Setstate "NewEnumerator0")
          (else
            (CallFunction|SetNewLocation)))
        (else
          (Transformation|SetActorLocation (+ _returnvalue _returnvalue_5) false false))))))

(fn ConstructionScript)

(fn Moveto
  (params (P :type Array%20of%20Vector%202D%20Int%20Structures))
  (bind _output_get (Variables|Default|SetPath P))
  (Utilities|Array|RemoveIndex _output_get (Utilities|Array|LastIndex _output_get))
  (Variables|Default|SetPathPos (- (Utilities|Array|Length _output_get) 1))
  (Variables|Default|Setstate "NewEnumerator1")
  (CallFunction|SetNewLocation))

(fn SetNewLocation
  (bind _outactors (Actor|GetAllActorsOfClass "/Game/Blueprints/BPWorldGrid.BPWorldGrid_C"))
  (Variables|Default|SetNext%20location (.location (Default|Vector2DInttoWorldTransform (Utilities|Array|Get(acopy) _outactors) (Utilities|Array|Get(acopy) (Variables|Default|GetPath) (Variables|Default|GetPathPos))))))